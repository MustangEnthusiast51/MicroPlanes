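; P-40E aircraft Blueprint, a child of a shared aircraft base that supplies its behavior.
; Tick, physics tick, input, camera, damage and hit events, plus the velocity and environment queries, pass straight through to the parent.
; Weapon firing also calls the parent, specifying the machine gun as the weapon.
; An unconnected leftover fragment rotates the cockpit camera from the mesh's angular velocity and never runs.
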(event `self.ReceiveTick`
  (params (DeltaSeconds :type "Float (single-precision)"))
  (`parent.ReceiveTick` DeltaSeconds))

(event `self.ReceiveAsyncPhysicsTick`
  (params (DeltaSeconds :type "Float (single-precision)") (SimSeconds :type "Float (single-precision)"))
  (`parent.ReceiveAsyncPhysicsTick` DeltaSeconds SimSeconds))

(event `SimpleFlightInterface.SetInputChannel`
  (params (channel :type Integer) (value :type "Float (single-precision)"))
  (`parent.SetInputChannel` channel value))

(event `SimpleFlightInterface.SetCameraDirectionValues`
  (params (directionalValues :type "Vector Structure"))
  (`parent.SetCameraDirectionValues` directionalValues))

(event `SimpleWeaponsInterface.FireWeapons`
  (params (triggered :type Boolean) (weapon :type "EWeaponType Enum" :default "MachineGun"))
  (`parent.FireWeapons` triggered "MachineGun"))

(event `SimpleWeaponsInterface.TakeHitDamage`
  (params (pos :type "Vector Structure") (damage :type "Float (single-precision)") (hit :type "HitResult Structure"))
  (`parent.TakeHitDamage` pos damage hit))

(event `self.ReceiveHit`
  (params (MyComp :type "PrimitiveComponent Object Reference") (Other :type "Actor Object Reference") (OtherComp :type "PrimitiveComponent Object Reference") (bSelfMoved :type Boolean) (HitLocation :type "Vector Structure") (HitNormal :type "Vector Structure") (NormalImpulse :type "Vector Structure") (Hit :type "HitResult Structure (by ref)"))
  (`parent.ReceiveHit` MyComp null null false (0.0 0.0 0.0) (0.0 0.0 0.0) (0.0 0.0 0.0) Hit))

(fn `GetEnvironmentData`
  (returns (ReturnValue :type "EnvironmentData Structure"))
  (bind _returnvalue (`parent.GetEnvironmentData`))
  (return _returnvalue))

(fn `GetInputChannel`
  (params (channel :type Integer))
  (returns (ReturnValue :type "Float (single-precision)"))
  (bind _returnvalue (`parent.GetInputChannel` channel))
  (return _returnvalue))

(fn `UserConstructionScript`
  (`parent.UserConstructionScript`))

(fn `VelocityAtPoint`
  (params (worldPos :type "Vector Structure"))
  (returns (ReturnValue :type "Vector Structure"))
  (bind _returnvalue (`parent.VelocityAtPoint` worldPos))
  (return _returnvalue))