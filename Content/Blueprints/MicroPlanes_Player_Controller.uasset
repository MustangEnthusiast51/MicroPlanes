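; Player controller for MicroPlanes that relays flight and camera input to any controlled pawn implementing SimpleFlightInterface.
; BeginPlay shows the cursor and adds the Enhanced Input mapping context, whose actions set roll, pitch, yaw and power channels.
; With MouseControl on, those flight actions are ignored; Tick instead maps viewport cursor position to roll and pitch, and integrates mouse wheel input into clamped power.
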(event `EnhancedInput|/SimpleFlight/Inputs/Camera_Vertical`
  (params (ActionValue :type "Float (double-precision)") (ElapsedSeconds :type "Float (double-precision)") (TriggeredSeconds :type "Float (double-precision)") (InputAction :type "InputAction Object Reference" :default "/SimpleFlight/Inputs/Camera_Vertical.Camera_Vertical"))
  (bind _returnvalue (`self.K2_GetPawn`))
  (:`Triggered`
    (if (`KismetSystemLibrary.DoesImplementInterface` _returnvalue "/Script/SimpleFlight.SimpleFlightInterface") :!label _label
      (message `SimpleFlightInterface.SetCameraDirectionValues` _returnvalue (`KismetMathLibrary.MakeVector` 0.0 ActionValue (stale `EnhancedInput|/SimpleFlight/Inputs/Camera_Horizontal` ActionValue)))))
  (:`Completed`
    (goto _label)))

(event `EnhancedInput|/SimpleFlight/Inputs/Camera_Horizontal`
  (params (ActionValue :type "Float (double-precision)") (ElapsedSeconds :type "Float (double-precision)") (TriggeredSeconds :type "Float (double-precision)") (InputAction :type "InputAction Object Reference" :default "/SimpleFlight/Inputs/Camera_Horizontal.Camera_Horizontal"))
  (:`Triggered`
    (goto _label))
  (:`Completed`
    (goto _label)))

(event `EnhancedInput|/SimpleFlight/Inputs/Power`
  (params (ActionValue :type "Float (double-precision)") (ElapsedSeconds :type "Float (double-precision)") (TriggeredSeconds :type "Float (double-precision)") (InputAction :type "InputAction Object Reference" :default "/SimpleFlight/Inputs/Power.Power"))
  (bind _returnvalue (`self.K2_GetPawn`))
  (:`Triggered`
    (if (`self.Mouse Control`) :!label _label_2
      _
      (elif (`KismetSystemLibrary.DoesImplementInterface` _returnvalue "/Script/SimpleFlight.SimpleFlightInterface")
        (message `SimpleFlightInterface.SetInputChannel` _returnvalue 3 ActionValue))))
  (:`Completed`
    (goto _label_2)))

(event `EnhancedInput|/SimpleFlight/Inputs/Yaw`
  (params (ActionValue :type "Float (double-precision)") (ElapsedSeconds :type "Float (double-precision)") (TriggeredSeconds :type "Float (double-precision)") (InputAction :type "InputAction Object Reference" :default "/SimpleFlight/Inputs/Yaw.Yaw"))
  (bind _returnvalue (`self.K2_GetPawn`))
  (:`Triggered`
    (if (`self.Mouse Control`) :!label _label_3
      _
      (elif (`KismetSystemLibrary.DoesImplementInterface` _returnvalue "/Script/SimpleFlight.SimpleFlightInterface")
        (message `SimpleFlightInterface.SetInputChannel` _returnvalue 2 ActionValue))))
  (:`Completed`
    (goto _label_3)))

(event `EnhancedInput|/SimpleFlight/Inputs/Roll`
  (params (ActionValue :type "Float (double-precision)") (ElapsedSeconds :type "Float (double-precision)") (TriggeredSeconds :type "Float (double-precision)") (InputAction :type "InputAction Object Reference" :default "/SimpleFlight/Inputs/Roll.Roll"))
  (bind _returnvalue (`self.K2_GetPawn`))
  (:`Triggered`
    (if (`self.Mouse Control`) :!label _label_4
      _
      (elif (`KismetSystemLibrary.DoesImplementInterface` _returnvalue "/Script/SimpleFlight.SimpleFlightInterface")
        (message `SimpleFlightInterface.SetInputChannel` _returnvalue 0 ActionValue))))
  (:`Completed`
    (goto _label_4)))

(event `EnhancedInput|/SimpleFlight/Inputs/Pitch`
  (params (ActionValue :type "Float (double-precision)") (ElapsedSeconds :type "Float (double-precision)") (TriggeredSeconds :type "Float (double-precision)") (InputAction :type "InputAction Object Reference" :default "/SimpleFlight/Inputs/Pitch.Pitch"))
  (bind _returnvalue (`self.K2_GetPawn`))
  (:`Triggered`
    (if (`self.Mouse Control`) :!label _label_5
      _
      (elif (`KismetSystemLibrary.DoesImplementInterface` _returnvalue "/Script/SimpleFlight.SimpleFlightInterface")
        (message `SimpleFlightInterface.SetInputChannel` _returnvalue 1 ActionValue))))
  (:`Completed`
    (goto _label_5)))

(event `self.ReceiveBeginPlay`
  (set `self.bShowMouseCursor` true)
  (`EnhancedInputSubsystemInterface.AddMappingContext` (pcsubsystem `EnhancedInputLocalPlayerSubsystem` self) "/SimpleFlight/Inputs/SimpleFlight_MappingContext.SimpleFlight_MappingContext" 0 (make `ModifyContextOptions` true)))

(event `self.ReceiveTick`
  (params (DeltaSeconds :type "Float (single-precision)"))
  (bind (_returnvalue_x _returnvalue_y) (`KismetMathLibrary.BreakVector2D` (`WidgetLayoutLibrary.GetViewportSize`)))
  (bind _returnvalue (`self.K2_GetPawn`))
  (bind (_locationx _locationy) (`self.GetMousePosition`))
  (if (`self.Mouse Control`)
    (if (`KismetSystemLibrary.DoesImplementInterface` (`self.K2_GetPawn`) "/Script/SimpleFlight.SimpleFlightInterface")
      (message `SimpleFlightInterface.SetInputChannel` _returnvalue 0 (`KismetMathLibrary.FClamp` (* (+ (/ _locationx _returnvalue_x) -0.5) 2.0) -1.0))
      (message `SimpleFlightInterface.SetInputChannel` _returnvalue 1 (`KismetMathLibrary.FClamp` (* (+ (/ _locationy _returnvalue_y) -0.5) 2.0) -1.0))
      (bind _returnvalue_2 (message `SimpleFlightInterface.GetInputChannel` _returnvalue 3))
      (message `SimpleFlightInterface.SetInputChannel` _returnvalue 3 (`KismetMathLibrary.FClamp` (+ _returnvalue_2 (* (stale `InputAxisKey|MouseWheelAxis` AxisValue) (`GameplayStatics.GetWorldDeltaSeconds`) 3.0)) 0.0)))))

(event `InputAxisKey|MouseWheelAxis`
  (params (AxisValue :type "Float (single-precision)")))

(fn `UserConstructionScript`)